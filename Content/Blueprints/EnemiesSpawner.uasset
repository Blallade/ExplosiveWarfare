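; EnemiesSpawner is a Blueprint that spawns a Grenadier enemy at a randomized location when its SpawnEnemy event runs and the SpawnEnemy flag is true.
; A two-pass loop is set up to roll X and Y offsets within a mirrored side range, with Z fixed at FloorHeight.
; Its index check is always true, so only X is randomized and the Y branch never runs.
; The spawn ignores collisions.
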(event `SpawnEnemy`
  (bind _randomareasiderange (`self.randomAreaSideRange`))
  (bind _returnvalue (`KismetMathLibrary.RandomFloatInRange` _randomareasiderange (* _randomareasiderange -1.0)))
  ;[0 1 1] Spawn enemy event
  (if (`self.spawnEnemy?`)
    (for _index (range 2)
      (if (>= _index 0)
        (set `self.XrandomSide` _returnvalue)
        (else
          (set `self.YrandomSide` _returnvalue))))
    (bind _output_get (set `self.randomSpawnLocation` (`KismetMathLibrary.MakeVector` (`self.XrandomSide`) (`self.YrandomSide`) (`self.floorHeight`))))
    (`|SpawnActorFromClass` "/Game/Blueprints/Grenadier.Grenadier_C" (`KismetMathLibrary.MakeTransform` _output_get) "AlwaysSpawn" "OverrideRootScale" null false null)))

(fn `UserConstructionScript`)