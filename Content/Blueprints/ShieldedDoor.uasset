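; Sliding door of a shielded room that seals the player in and protects them from the orbital bombardment.
; The first player overlap of its Box stops the room's UI advice, plays a sound and runs a timeline that lerps the door along Y.
; When the timeline finishes, it flags the player as shielded on OrbitalBombardment.
; OpenDoor, noted as triggered by a full special bar, reverses that timeline once with the same sound.
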(event `self.Box.OnComponentBeginOverlap`
  (params (OverlappedComponent :type "PrimitiveComponent Object Reference") (OtherActor :type "Actor Object Reference") (OtherComp :type "PrimitiveComponent Object Reference") (OtherBodyIndex :type Integer) (bFromSweep :type Boolean) (SweepResult :type "HitResult Structure (by ref)"))
  (bind (_returnvalue_x _returnvalue_y _returnvalue_z) (`KismetMathLibrary.BreakVector` (`self.K2_GetActorLocation`)))
  ;[0 0.4984 1] Shields character when he goes into shielded room
  (cast `/Game/Blueprints/FirstPersonCharacter` OtherActor)
  (`/Engine/EditorBlueprintResources/StandardMacros.DoOnce` false
    (:`Completed`
      (bind _foundwidgets (`WidgetBlueprintLibrary.GetAllWidgetsOfClass` "/Game/Blueprints/Widgets/PlayerUI.PlayerUI_C"))
      (`/Game/Blueprints/Widgets/PlayerUI.StopShieldedRoomAdviceUI` (`|GetArrayItem` _foundwidgets))
      (set `self.shielded?` true)
      (`GameplayStatics.SpawnSoundAtLocation` "/Game/Audio/Door_Moving.Door_Moving" (`KismetMathLibrary.MakeVector` _returnvalue_x _returnvalue_y _returnvalue_z) (struct) 0.3 2.0 0.0 null null)
      (bind (_direction _alpha) (`Timeline|DoorClosingAnim` :!via `PlayFromStart` :!label _label)
        (:`Update`
          (`self.K2_SetActorLocation` (`KismetMathLibrary.MakeVector` _returnvalue_x (`KismetMathLibrary.Lerp` (`self.YFirstLocation`) (`self.YLastLocation`) _alpha) _returnvalue_z)))
        (:`Finished`
          (if (`self.shielded?`)
            (bind _returnvalue (`GameplayStatics.GetActorOfClass` "/Game/Blueprints/OrbitalBombardment.OrbitalBombardment_C"))
            (set `/Game/Blueprints/OrbitalBombardment.isPlayerShielded?` true _returnvalue)))))))

(event `OpenDoor`
  (bind (_returnvalue_x _returnvalue_y _returnvalue_z) (`KismetMathLibrary.BreakVector` (`self.K2_GetActorLocation`)))
  ;[0 0.4984 1] Shields character when he goes into shielded room
  ;;[1 0.05208 1] Opens the door when fills the special bar
  (`/Engine/EditorBlueprintResources/StandardMacros.DoOnce` false
    (:`Completed`
      (`GameplayStatics.SpawnSoundAtLocation` "/Game/Audio/Door_Moving.Door_Moving" (`KismetMathLibrary.MakeVector` _returnvalue_x _returnvalue_y _returnvalue_z) (struct) 0.3 2.0 0.0 null null)
      (goto _label :!via `ReverseFromEnd`))))

(fn `UserConstructionScript`)