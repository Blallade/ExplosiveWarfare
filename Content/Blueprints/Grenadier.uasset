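; Grenadier enemy that turns to face the player and periodically throws grenades from its right hand.
; After a random initial delay, a repeating loop sets an attack flag and spawns a grenade, provided both it and the player are alive.
; Damage lowers clamped HP and plays a hit sound.
; Death runs once, asks the EnemiesSpawner for a new enemy, disables collision, then sinks the corpse via timeline before destroying it.
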(event `self.ReceiveTick`
  (params (DeltaSeconds :type "Float (single-precision)"))
  ;[0.6771 0.3168 0.04937] Focus character effect and checks character life
  (if (<= (`self.currentHP`) 0.0)
    (`self.DeathEvent`)
    (else
      (`self.K2_SetActorRotation` (`KismetMathLibrary.FindLookAtRotation` (`self.K2_GetActorLocation`) (`self.K2_GetActorLocation` (`GameplayStatics.GetPlayerCharacter` 0)))))))

(event `self.ReceiveBeginPlay`
  ;[0.2492 0.2292 1] Throw grenade cycle
  (`KismetSystemLibrary.Delay` (`KismetMathLibrary.RandomFloatInRange` 1.0 5.0))
  (`self.ThrowGrenade` :!label _label)
  (`KismetSystemLibrary.Delay` 5.0)
  (goto _label))

(event `DeathEvent`
  (bind (_returnvalue_x _returnvalue_y _returnvalue_z) (`KismetMathLibrary.BreakVector` (`self.K2_GetActorLocation`)))
  (bind (_returnvalue_x_2 _returnvalue_y_2) (`KismetMathLibrary.BreakVector` (`self.K2_GetActorLocation`)))
  (bind _zlocation (`self.ZLocation`))
  ;[0.09375 0 0] Death event
  (`/Engine/EditorBlueprintResources/StandardMacros.DoOnce` false
    (:`Completed`
      (set `self.ZLocation` _returnvalue_z)
      (`GameplayStatics.PlaySoundAtLocation` "/Game/Audio/Bones_Death.Bones_Death" (`KismetMathLibrary.MakeVector` _returnvalue_x _returnvalue_y _returnvalue_z) (struct) 1.0 1.0 0.0 null null null)
      (set `self.isAlive?` false)
      (bind _returnvalue (`GameplayStatics.GetActorOfClass` "/Game/Blueprints/EnemiesSpawner.EnemiesSpawner_C"))
      (`/Game/Blueprints/EnemiesSpawner.SpawnEnemy` _returnvalue)
      (`PrimitiveComponent.SetCollisionEnabled` (`self.Collision`) "NoCollision")
      (`KismetSystemLibrary.Delay` 3.0)
      ;;[0.8854 0.4182 0.07378] Earth swallowing corpse animation
      (bind (_direction _alpha) (`Timeline|DeathAnim` :!via `PlayFromStart`)
        (:`Update`
          (`self.K2_SetActorLocation` (`KismetMathLibrary.MakeVector` _returnvalue_x_2 _returnvalue_y_2 (`KismetMathLibrary.Lerp` _zlocation (- _zlocation 100.0) _alpha))))
        (:`Finished`
          (`self.K2_DestroyActor`))))))

(event `ThrowGrenade`
  ;[0 1 1] Throw grenade event
  (if (`self.isAlive?`)
    (if (not (`/Game/Blueprints/FirstPersonCharacter.dead?` (cast `/Game/Blueprints/FirstPersonCharacter` (`GameplayStatics.GetPlayerCharacter` 0) :!pure true)))
      (set `self.isAttacking?` true)
      (`KismetSystemLibrary.Delay` 0.7)
      (if (`self.isAlive?`)
        (`|SpawnActorFromClass` "/Game/Blueprints/Grenade.Grenade_C" (`SceneComponent.K2_GetComponentToWorld` (`self.RightHand`)) "AlwaysSpawn" "OverrideRootScale" null null)
        (`KismetSystemLibrary.Delay` 0.5)
        (set `self.isAttacking?` false)))))

(event `ReceiveDmg`
  (params (`dmgReceived?` :type "Float (double-precision)"))
  ;[0.1667 1 0.1995] Receive damage event
  (bind _output_get (set `self.currentHP` (`KismetMathLibrary.FClamp` (- (`self.currentHP`) `dmgReceived?`) 0.0 100.0)))
  (if (<= _output_get 0.0)
    (`self.DeathEvent`)
    (else
      (`GameplayStatics.SpawnSoundAtLocation` "/Game/Audio/Bones_Hit.Bones_Hit" (`self.K2_GetActorLocation`) (struct) 0.4 1.3 0.0 null null))))

(fn `UserConstructionScript`)