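; Orbital bombardment actor that drops a bomb from high altitude and triggers a scripted, level-wide explosion.
; ThrowBomb plays an alert and wind sound, then after a delay a timeline lowers the actor while the wind grows louder.
; On impact it spawns explosion effects, switches off the LightBar, breaks WindowGlass and stops the main music.
; It damages every Grenadier and the player, passing along whether the player is shielded.
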(event `ThrowBomb`
  ;[0.1541 0 0.6979] Throw bomb effects
  (bind _returnvalue (`GameplayStatics.SpawnSound2D` "/Game/Audio/Bomb_alert.Bomb_alert" 0.2 1.0 0.0 null))
  (`AudioComponent.FadeIn` _returnvalue 1.0 1.0 0.0 "Linear")
  (bind _returnvalue_2 (`GameplayStatics.SpawnSoundAtLocation` "/Game/Audio/Wind.Wind" (`self.K2_GetActorLocation`) (struct) 0.1 1.0 0.0 null null))
  (set `self.windSound` _returnvalue_2)
  (`KismetSystemLibrary.Delay` 5.0)
  (`self.BombFall`))

(event `BombFall`
  (bind _returnvalue (`self.K2_GetActorLocation`))
  ;[1 0.0625 1] Bomb fall
  (`AudioComponent.AdjustVolume` (`self.windSound`) 8.0 4.0 "Linear")
  (bind (_direction _alpha) (`Timeline|BombFallAnim` :!via `PlayFromStart`)
    (:`Update`
      (`self.K2_SetActorLocation` (`KismetMathLibrary.MakeVector` 0.0 0.0 (`KismetMathLibrary.Lerp` 20000.0 5.0 _alpha))))
    (:`Finished`
      ;[0.2656 0.01771 0] Bomb impact
      (`AudioComponent.FadeOut` (`self.windSound`) 0.3 0.0 "Linear")
      (`GameplayStatics.SpawnSound2D` "/Game/Audio/Orbital_bombarment_explosion.Orbital_bombarment_explosion" 0.5 1.0 0.0 null)
      (`ActorComponent.K2_DestroyComponent` (`self.StaticMesh`))
      (`GameplayStatics.SpawnEmitterAtLocation` "/Game/ThirdParty/StarterContent/Particles/P_Explosion.P_Explosion" _returnvalue (struct) (40.0 40.0 40.0))
      (`GameplayStatics.SpawnEmitterAtLocation` "/Game/ThirdParty/StarterContent/Particles/P_Smoke.P_Smoke" _returnvalue (struct) (40.0 40.0 40.0))
      (bind _returnvalue_2 (`GameplayStatics.GetActorOfClass` "/Game/Blueprints/LightBar.LightBar_C"))
      (`/Game/Blueprints/LightBar.TurnOffLights` _returnvalue_2)
      (bind _returnvalue_3 (`GameplayStatics.GetActorOfClass` "/Game/Blueprints/WindowGlass.WindowGlass_C"))
      (`/Game/Blueprints/WindowGlass.BreakGlass` _returnvalue_3)
      (bind _outactors (`GameplayStatics.GetAllActorsOfClass` "/Game/Blueprints/Grenadier.Grenadier_C"))
      (for _array_element _outactors
        (`/Game/Blueprints/Grenadier.ReceiveDmg` _array_element (`self.missileDmg`)))
      (`/Game/Blueprints/FirstPersonCharacter.ReceiveBombDmg` (cast `/Game/Blueprints/FirstPersonCharacter` (`GameplayStatics.GetPlayerCharacter` 0) :!pure true) (`self.isPlayerShielded?`) (`self.missileDmg`))
      (bind _returnvalue_4 (`GameplayStatics.GetActorOfClass` "/Game/Blueprints/MusicManager.MusicManager_C"))
      (`/Game/Blueprints/MusicManager.StopMainTheme` _returnvalue_4))))

(fn `UserConstructionScript`)