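; LightBar is a light fixture Blueprint with a rect light and a glowing mesh that can be switched off with a bulb-break effect.
; Its TurnOffLights event plays a timeline that fades the light by repeatedly lerping its current intensity toward zero.
; When the timeline finishes, a DoOnce swaps the mesh materials to the unlit glow variant and spawns the bulb-break sound at the actor's location.
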(event `TurnOffLights`
  (bind _staticmeshcomponent (`self.StaticMeshComponent`))
  (bind _rectlight (`self.RectLight`))
  ;[1 0.3959 0.0599] Turns off the lights and sets the Lightbar materials
  (bind (_direction _alpha) (`Timeline|TurnOffLightsSpeed`)
    (:`Update`
      (`LightComponent.SetIntensity` _rectlight (`KismetMathLibrary.Lerp` (`LightComponentBase.Intensity` _rectlight) 0.0 _alpha)))
    (:`Finished`
      (`/Engine/EditorBlueprintResources/StandardMacros.DoOnce` false
        (:`Completed`
          (`PrimitiveComponent.SetMaterial` _staticmeshcomponent 0 "/Game/Materials/MI_GlowLightOff.MI_GlowLightOff")
          (`PrimitiveComponent.SetMaterial` _staticmeshcomponent 1 "/Game/Materials/MI_GlowLightOff.MI_GlowLightOff")
          (`PrimitiveComponent.SetMaterial` _staticmeshcomponent 2 "/Game/Materials/MI_GlowLightOff.MI_GlowLightOff")
          (`GameplayStatics.SpawnSoundAtLocation` "/Game/Audio/Bulb_Break.Bulb_Break" (`self.K2_GetActorLocation`) (struct) 1.0 1.0 0.0 null null))))))

(fn `UserConstructionScript`)