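; Grenade actor that explodes on impact and damages a FirstPersonCharacter within its damage collision.
; The damage collision stays disabled until the first hit, which spawns an explosion emitter, enables query-only overlap and immediately destroys the actor.
; Overlap passes GrenadeDmg to the character's ReceiveDmg, with a DoOnce limiting damage to the first character detected.
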(event `self.ReceiveBeginPlay`
  ;[0 0.1431 0.5885] Sets the radius damage collision to false at the beginning
  (`PrimitiveComponent.SetCollisionEnabled` (`self.DmgCollision`) "NoCollision"))

(event `self.Collision.OnComponentHit`
  (params (HitComponent :type "PrimitiveComponent Object Reference") (OtherActor :type "Actor Object Reference") (OtherComp :type "PrimitiveComponent Object Reference") (NormalImpulse :type "Vector Structure") (Hit :type "HitResult Structure (by ref)"))
  ;[1 0.02745 0.2314] On grenade hits collision
  (`/Engine/EditorBlueprintResources/StandardMacros.DoOnce` false
    (:`Completed`
      (`GameplayStatics.SpawnEmitterAtLocation` "/Game/ThirdParty/StarterContent/Particles/P_Explosion.P_Explosion" (`self.K2_GetActorLocation`) (struct) (2.0 2.0 2.0))
      (`PrimitiveComponent.SetCollisionEnabled` (`self.DmgCollision`) "QueryOnly")
      (`self.K2_DestroyActor`))))

(event `self.DmgCollision.OnComponentBeginOverlap`
  (params (OverlappedComponent :type "PrimitiveComponent Object Reference") (OtherActor :type "Actor Object Reference") (OtherComp :type "PrimitiveComponent Object Reference") (OtherBodyIndex :type Integer) (bFromSweep :type Boolean) (SweepResult :type "HitResult Structure (by ref)"))
  ;[1 0.02745 0.2314] On grenade damage collision
  (bind _asfirst_person_character (cast `/Game/Blueprints/FirstPersonCharacter` OtherActor))
  (`/Engine/EditorBlueprintResources/StandardMacros.DoOnce` false
    (:`Completed`
      (`/Game/Blueprints/FirstPersonCharacter.ReceiveDmg` _asfirst_person_character (`self.grenadeDmg`)))))

(fn `UserConstructionScript`)